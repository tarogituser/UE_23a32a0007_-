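; BP_PointItem is a pickup that awards points to the actor touching it.
; A Rotate timeline started at BeginPlay drives the yaw of its static mesh, resetting the stored angle once it reaches 360 degrees.
; When an actor begins overlapping its Box, it sends that actor a CharacterHitActionMessage carrying the Point value, then destroys itself.
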(event `self.ReceiveBeginPlay`
  (bind (_direction _rotation) (`Timeline|Rotate`)
    (:`Update`
      (if (< (`self.ActorRotation`) 360.0)
        (set `self.ActorRotation` _rotation)
        (else
          (set `self.ActorRotation` 0.0)))
      (`SceneComponent.K2_SetRelativeRotation` (`self.STM_PointItem`) (`KismetMathLibrary.MakeRotator` 0.0 0.0 (`self.ActorRotation`)) false false))))

(event `self.Box.OnComponentBeginOverlap`
  (params (OverlappedComponent :type "PrimitiveComponent Object Reference") (OtherActor :type "Actor Object Reference") (OtherComp :type "PrimitiveComponent Object Reference") (OtherBodyIndex :type Integer) (bFromSweep :type Boolean) (SweepResult :type "HitResult Structure (by ref)"))
  (message `/Game/Project/BluePrints/BPI_MyCharacter.CharacterHitAction` OtherActor (`self.Point`))
  (`self.K2_DestroyActor`))

(fn `UserConstructionScript`)